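; BP_WindSource is an actor that repeatedly relocates itself to random points at a fixed height, apparently serving as a moving wind origin.
; A slowed timeline starts on BeginPlay and, each time it finishes, picks new random locations and replays.
; Timeline updates set the actor directly to the next location without interpolation, so it jumps rather than glides, and the stored start location goes unused.
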(event EventBeginPlay
  (Components|Timeline|SetPlayRate (Variables|Default|GetRandomize%20Wind%20Source%20Location) 0.2)
  (Variables|Default|SetWindSourceStartLoc (Math|Vector|MakeVector (Math|Random|RandomFloatinRange -1e+04 1e+04) (Math|Random|RandomFloatinRange -1e+04 1e+04) 1e+03) :!label _label)
  (Variables|Default|SetWindSourceNextLoc (Math|Vector|MakeVector (Math|Random|RandomFloatinRange -1e+04 1e+04) (Math|Random|RandomFloatinRange -1e+04 1e+04) 1e+03))
  (Timeline|Randomize%20Wind%20Source%20Location PlayFromStart
    (:Update
      (Transformation|SetActorLocation (Variables|Default|GetWindSourceNextLoc) false false))
    (:Finished
      (goto _label))))

(fn ConstructionScript)