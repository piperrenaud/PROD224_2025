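; Player controller for a helicopter, turning Enhanced Input actions into control flags and driving vertical flight of the possessed BP_Helicopter.
; Each Tick, the lift flag selects climb or fall, accelerating a shared, clamped speed that offsets the HeliPivot's relative Z.
; Engine toggle and forward, left and right inputs only set flags; their movement and engine functions are empty, and lift ignores engine state.
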(event Input|EnhancedActionEvents|EnhancedInputActionIA_EngineOn
  (params (ActionValue :type Boolean) (ElapsedSeconds :type Float%20%28double-precision%29) (TriggeredSeconds :type Float%20%28double-precision%29) (InputAction :type Input%20Action%20Object%20Reference :default "/Game/InputActions/IA_EngineOn.IA_EngineOn"))
  ;[0.15 0.15 0.15 0.5] EngineOn button On/Off detection
  (Utilities|FlowControl|FlipFlop
    (:A
      (Variables|Default|SetIsEngineOn true))
    (:B
      (Variables|Default|SetIsEngineOn false))))

(event Input|EnhancedActionEvents|EnhancedInputActionIA_LiftUp
  (params (ActionValue :type Boolean) (ElapsedSeconds :type Float%20%28double-precision%29) (TriggeredSeconds :type Float%20%28double-precision%29) (InputAction :type Input%20Action%20Object%20Reference :default "/Game/InputActions/IA_LiftUp.IA_LiftUp"))
  ;[0.15 0.15 0.15 0.5] LiftUp Button press detection
  (:Triggered
    (Variables|Default|SetIsLifting true))
  (:Completed
    (Variables|Default|SetIsLifting false)))

(event Input|EnhancedActionEvents|EnhancedInputActionIA_MoveForward
  (params (ActionValue :type Float%20%28double-precision%29) (ElapsedSeconds :type Float%20%28double-precision%29) (TriggeredSeconds :type Float%20%28double-precision%29) (InputAction :type Input%20Action%20Object%20Reference :default "/Game/InputActions/IA_MoveForward.IA_MoveForward"))
  ;[0.15 0.15 0.15 0.5] MoveForward button press detection
  (:Triggered
    (Variables|Default|SetIsMovingForward true))
  (:Completed
    (Variables|Default|SetIsMovingForward false)))

(event Input|EnhancedActionEvents|EnhancedInputActionIA_MoveLeft
  (params (ActionValue :type Boolean) (ElapsedSeconds :type Float%20%28double-precision%29) (TriggeredSeconds :type Float%20%28double-precision%29) (InputAction :type Input%20Action%20Object%20Reference :default "/Game/InputActions/IA_MoveLeft.IA_MoveLeft"))
  ;[0.15 0.15 0.15 0.5] MoveLeft button press detection
  (:Triggered
    (Variables|Default|SetIsMovingLeft true))
  (:Completed
    (Variables|Default|SetIsMovingLeft false)))

(event Input|EnhancedActionEvents|EnhancedInputActionIA_MoveRight
  (params (ActionValue :type Boolean) (ElapsedSeconds :type Float%20%28double-precision%29) (TriggeredSeconds :type Float%20%28double-precision%29) (InputAction :type Input%20Action%20Object%20Reference :default "/Game/InputActions/IA_MoveRight.IA_MoveRight"))
  ;[0.15 0.15 0.15 0.5] MoveRight button press detection
  (:Triggered
    (Variables|Default|SetIsMovingRight true))
  (:Completed
    (Variables|Default|SetIsMovingRight false)))

(event EventBeginPlay
  ;[0.15 0.15 0.15 0.5] Cast to Helicopter BP
  (bind _asbp_helicopter (Utilities|Casting|CastToBP_Helicopter (Pawn|GetControlledPawn)))
  (Variables|Default|SetHeliPivot (Variables|/Game/Blueprints/BP_Helicopter.BP_Helicopter_C|GetHeliPivot _asbp_helicopter)))

(event EventTick
  (params (DeltaSeconds :type Float%20%28single-precision%29))
  ;[0.15 0.15 0.15 0.5] Call Functions
  (if (Variables|Default|GetIsLifting)
    (CallFunction|MoveUpwards)
    (else
      (CallFunction|MoveDownwards))))

(fn ConstructionScript)

(fn Engineon
  (params (IsPressed :type Boolean)))

(fn MoveUpwards
  (bind _helipivot (Variables|Default|GetHeliPivot))
  (bind _relativelocation (Variables|/Script/Engine.SceneComponent|GetRelativeLocation _helipivot))
  (bind _output_get (Variables|Default|SetCurrentLiftSpeed (Math|Float|Clamp(Float) (+ (Variables|Default|GetCurrentLiftSpeed) (* (Variables|Default|GetLiftAcceleration) (Utilities|Time|GetWorldDeltaSeconds))) 0.0 (Variables|Default|GetMaxLiftSpeed))))
  (Transformation|SetRelativeLocation (Variables|Default|GetHeliPivot) (Math|Vector|MakeVector (.x _relativelocation) (.y _relativelocation) (+ _output_get (.z _relativelocation))) false false))

(fn MoveDownwards
  (bind _helipivot (Variables|Default|GetHeliPivot))
  (bind _relativelocation (Variables|/Script/Engine.SceneComponent|GetRelativeLocation _helipivot))
  (bind _output_get (Variables|Default|SetCurrentLiftSpeed (Math|Float|Clamp(Float) (+ (Variables|Default|GetCurrentLiftSpeed) (* (Variables|Default|GetGravityAcceleration) (Utilities|Time|GetWorldDeltaSeconds))) (Variables|Default|GetMaxGravitySpeed) 0.0)))
  (Transformation|SetRelativeLocation (Variables|Default|GetHeliPivot) (Math|Vector|MakeVector (.x _relativelocation) (.y _relativelocation) (+ _output_get (.z _relativelocation))) false false))

(fn MoveForward
  (params (Force :type Float%20%28double-precision%29)))

(fn MoveLeft)

(fn MoveRight)