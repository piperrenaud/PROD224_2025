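; Helipad actor that changes the color of its four point lights to show how close the player's helicopter is.
; On BeginPlay it casts the player pawn to BP_Helicopter and caches its HeliPivot component.
; Each Tick it measures the distance from that pivot to PadController and sets the lights green, orange or red as the helicopter gets nearer, leaving them unchanged outside those bands.
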(event EventBeginPlay
  ;[0.15 0.15 0.15 0.5] HeliPivot Reference
  (bind _asbp_helicopter (Utilities|Casting|CastToBP_Helicopter (Game|Player|GetPlayerPawn 0)))
  (Variables|Default|SetHeli%20Pivot (Variables|/Game/Blueprints/BP_Helicopter.BP_Helicopter_C|GetHeliPivot _asbp_helicopter)))

(event EventTick
  (params (DeltaSeconds :type Float%20%28single-precision%29))
  (bind _heli_pivot (Variables|Default|GetHeli%20Pivot))
  (bind _pad_controller (Variables|Default|GetPad%20Controller))
  (bind _returnvalue (Transformation|GetWorldLocation _pad_controller))
  (bind _returnvalue_2 (Transformation|GetWorldLocation _heli_pivot))
  (bind _returnvalue_3 (Math|Vector|Distance(Vector) _returnvalue_2 _returnvalue))
  ;[0.15 0.15 0.15 0.5] Find Distance
  (Utilities|FlowControl|Sequence
    (:then_0
      (if (Math|Float|InRange(Float) _returnvalue_3 1001.0 3e+03)
        ;[0.15 0.15 0.15 0.5] Light
        (Rendering|Components|Light|SetLightColor (Variables|Default|GetPointLight) "(R=0.061246,G=1.000000,B=0.000000,A=1.000000)" true)
        (Rendering|Components|Light|SetLightColor (Variables|Default|GetPointLight1) "(R=0.061246,G=1.000000,B=0.000000,A=1.000000)" true)
        (Rendering|Components|Light|SetLightColor (Variables|Default|GetPointLight2) "(R=0.061246,G=1.000000,B=0.000000,A=1.000000)" true)
        (Rendering|Components|Light|SetLightColor (Variables|Default|GetPointLight3) "(R=0.061246,G=1.000000,B=0.000000,A=1.000000)" true)))
    (:then_1
      (if (Math|Float|InRange(Float) _returnvalue_3 501.0 1e+03)
        (Rendering|Components|Light|SetLightColor (Variables|Default|GetPointLight) "(R=1.000000,G=0.445851,B=0.000000,A=1.000000)" true)
        (Rendering|Components|Light|SetLightColor (Variables|Default|GetPointLight1) "(R=1.000000,G=0.445851,B=0.000000,A=1.000000)" true)
        (Rendering|Components|Light|SetLightColor (Variables|Default|GetPointLight2) "(R=1.000000,G=0.445851,B=0.000000,A=1.000000)" true)
        (Rendering|Components|Light|SetLightColor (Variables|Default|GetPointLight3) "(R=1.000000,G=0.445851,B=0.000000,A=1.000000)" true)))
    (:then_2
      (if (Math|Float|InRange(Float) _returnvalue_3 0.0 5e+02)
        (Rendering|Components|Light|SetLightColor (Variables|Default|GetPointLight) "(R=1.000000,G=0.018362,B=0.000000,A=1.000000)" true)
        (Rendering|Components|Light|SetLightColor (Variables|Default|GetPointLight1) "(R=1.000000,G=0.018362,B=0.000000,A=1.000000)" true)
        (Rendering|Components|Light|SetLightColor (Variables|Default|GetPointLight2) "(R=1.000000,G=0.018362,B=0.000000,A=1.000000)" true)
        (Rendering|Components|Light|SetLightColor (Variables|Default|GetPointLight3) "(R=1.000000,G=0.018362,B=0.000000,A=1.000000)" true)))))

(fn ConstructionScript)