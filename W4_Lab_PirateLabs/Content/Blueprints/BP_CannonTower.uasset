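; Enemy cannon tower that tracks the player's pirate ship and fires cannonballs at it when it is within attack distance.
; BeginPlay caches the player pawn as the ship, then Tick runs FireCannon and LookAtPirateShip.
; FireCannon computes distance by hand and advances a cooldown only while in range, spawning a ball and smoke at the barrel end.
; LookAtPirateShip applies world look-at yaw as the pivot's relative rotation, without pitch.
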(event EventBeginPlay
  ;[0.2664 0.5647 0.2159 0.502] Acquire Var Refs
  (bind _asbp_pirate_ship (Utilities|Casting|CastToBP_PirateShip (Game|Player|GetPlayerPawn 0)))
  (Variables|Default|SetPirateShip _asbp_pirate_ship))

(event EventTick
  (params (DeltaSeconds :type Float%20%28single-precision%29))
  (CallFunction|FireCannon)
  (CallFunction|LookatPirateShip))

(fn ConstructionScript)

(fn FireCannon
  (bind _cannon_pivot (Variables|Default|GetCannon%20Pivot))
  (bind _cannon_barrel_end (Variables|Default|GetCannon%20Barrel%20End))
  (bind _pirateship (Variables|Default|GetPirateShip))
  (bind _returnvalue (Transformation|GetWorldLocation _cannon_pivot))
  (bind _returnvalue_2 (Transformation|GetActorLocation _pirateship))
  (bind _returnvalue_3 (Transformation|GetWorldTransform _cannon_barrel_end))
  (bind _returnvalue_4 (- _returnvalue_2 _returnvalue))
  (bind (_location _rotation) (Math|Transform|BreakTransform _returnvalue_3))
  (if (< (Math|Float|Sqrt (+ (Math|Float|Power (.x _returnvalue_4) 2.0) (Math|Float|Power (.y _returnvalue_4) 2.0) (Math|Float|Power (.z _returnvalue_4) 2.0))) (Variables|Default|GetAttackDistance))
    (bind _output_get (Variables|Default|SetCurrentCooldownTimer (+ (Variables|Default|GetCurrentCooldownTimer) (Utilities|Time|GetWorldDeltaSeconds))))
    (if (> _output_get (Variables|Default|GetFireCooldown))
      (Game|SpawnActorfromClass "/Game/Blueprints/BP_CannonBall.BP_CannonBall_C" _returnvalue_3 "Undefined" "OverrideRootScale" 0 0) ; Spawn a Cannon Ball
      (Effects|SpawnEmitteratLocation "/Game/Particles/P_CannonSmoke.P_CannonSmoke" _location _rotation "5.000000,5.000000,5.000000") ; Spawn Smoke Particles
      (Variables|Default|SetCurrentCooldownTimer 0.0) ; Reset Cooldown Timer
    )))

(fn LookatPirateShip
  (bind _cannon_pivot (Variables|Default|GetCannon%20Pivot))
  (Transformation|SetRelativeRotation _cannon_pivot (Math|Rotator|MakeRotator 0.0 0.0 (.Yaw (Math|Rotator|BreakRotator (Math|Rotator|FindLookatRotation (Transformation|GetWorldLocation _cannon_pivot) (Transformation|GetActorLocation (Variables|Default|GetPirateShip)))))) false false))