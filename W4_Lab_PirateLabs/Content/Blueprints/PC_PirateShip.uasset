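; Player controller for a sailing pirate ship: input turns the ship pivot and swings the three sail pivots.
; Each tick, MoveForward accelerates the ship along its forward vector up to a maximum speed.
; CatchWind sets that maximum and acceleration in three tiers, using the angle between normalized ship and wind-source world positions, ignoring heading and sails.
; DetermineWindSide is an empty stub, with disconnected wind-side labels noted as HUD-linked.
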(event Input|EnhancedActionEvents|EnhancedInputActionSailLeft
  (params (ActionValue :type Boolean) (ElapsedSeconds :type Float%20%28double-precision%29) (TriggeredSeconds :type Float%20%28double-precision%29) (InputAction :type Input%20Action%20Object%20Reference :default "/Game/Blueprints/SailLeft.SailLeft"))
  (bind _rearsailpivot (Variables|Default|GetRearSailPivot))
  ;[0.15 0.15 0.15 0.5] Sail Rotation
  (:Triggered
    (Transformation|SetRelativeRotation _rearsailpivot "0.000000,-40.000000,0.000000" false false))
  (:Completed
    (Transformation|SetRelativeRotation _rearsailpivot "0, 0, 0" false false)))

(event Input|EnhancedActionEvents|EnhancedInputActionSailRight
  (params (ActionValue :type Boolean) (ElapsedSeconds :type Float%20%28double-precision%29) (TriggeredSeconds :type Float%20%28double-precision%29) (InputAction :type Input%20Action%20Object%20Reference :default "/Game/Blueprints/SailRight.SailRight"))
  (bind _rearsailpivot (Variables|Default|GetRearSailPivot))
  ;[0.15 0.15 0.15 0.5] Sail Rotation
  (:Triggered
    (Transformation|SetRelativeRotation _rearsailpivot "0.000000,40.000000,0.000000" false false))
  (:Completed
    (Transformation|SetRelativeRotation _rearsailpivot "0, 0, 0" false false)))

(event Input|EnhancedActionEvents|EnhancedInputActionSteerLeft
  (params (ActionValue :type Boolean) (ElapsedSeconds :type Float%20%28double-precision%29) (TriggeredSeconds :type Float%20%28double-precision%29) (InputAction :type Input%20Action%20Object%20Reference :default "/Game/Blueprints/SteerLeft.SteerLeft"))
  ;[0.15 0.15 0.15 0.5] Ship Rotation
  (Transformation|AddRelativeRotation (Variables|Default|GetShipPivot) "0.000000,-1.000000,0.000000" false false))

(event Input|EnhancedActionEvents|EnhancedInputActionSteerRight
  (params (ActionValue :type Boolean) (ElapsedSeconds :type Float%20%28double-precision%29) (TriggeredSeconds :type Float%20%28double-precision%29) (InputAction :type Input%20Action%20Object%20Reference :default "/Game/Blueprints/SteerRight.SteerRight"))
  ;[0.15 0.15 0.15 0.5] Ship Rotation
  (Transformation|AddRelativeRotation (Variables|Default|GetShipPivot) "0.000000,1.000000,0.000000" false false))

(event EventBeginPlay
  (bind _returnvalue (Pawn|GetControlledPawn))
  ;[0.2664 0.5647 0.2159 0.502] Acquire Var Refs
  (Utilities|FlowControl|Sequence
    (:then_0
      (bind _asbp_pirate_ship (Utilities|Casting|CastToBP_PirateShip _returnvalue))
      (Variables|Default|SetShipPivot (Variables|/Game/Blueprints/BP_PirateShip.BP_PirateShip_C|GetShip%20Pivot _asbp_pirate_ship))
      (bind _asbp_pirate_ship_2 (Utilities|Casting|CastToBP_PirateShip _returnvalue))
      (Variables|Default|SetFrontSailPivot (Variables|/Game/Blueprints/BP_PirateShip.BP_PirateShip_C|GetFront%20Sail%20Pivot _asbp_pirate_ship_2))
      (Variables|Default|SetMiddleSailPivot (Variables|/Game/Blueprints/BP_PirateShip.BP_PirateShip_C|GetMiddle%20Sail%20Pivot _asbp_pirate_ship_2))
      (Variables|Default|SetRearSailPivot (Variables|/Game/Blueprints/BP_PirateShip.BP_PirateShip_C|GetRear%20Sail%20Pivot _asbp_pirate_ship_2)))
    (:then_1
      (bind _outactors (Actor|GetAllActorsOfClass "/Game/Blueprints/BP_WindSource.BP_WindSource_C"))
      (Variables|Default|SetWindSource (Utilities|Array|Get(acopy) _outactors))
      (bind _asbp_pirate_ship_3 (Utilities|Casting|CastToBP_PirateShip (Pawn|GetControlledPawn)))
      (Variables|Default|SetPirateShipHUD (Variables|/Game/Blueprints/BP_PirateShip.BP_PirateShip_C|GetPirateShipHUD _asbp_pirate_ship_3)))))

(event EventTick
  (params (DeltaSeconds :type Float%20%28single-precision%29))
  ;[0.138 0.2201 0.5 0.5] Main Game Loop
  (CallFunction|MoveForward)
  (CallFunction|CatchWind)
  (CallFunction|DetermineWindSide))

(fn ConstructionScript)

(fn MoveForward
  (bind _output_get (Variables|Default|SetCurrentForwardSpeed (Math|Float|Clamp(Float) (+ (Variables|Default|GetCurrentForwardSpeed) (* (Variables|Default|GetForwardAcceleration) (Utilities|Time|GetWorldDeltaSeconds))) 0.0 (Variables|Default|GetMaxForwardSpeed))))
  (Transformation|AddRelativeLocation (Variables|Default|GetShipPivot) (* _output_get (Math|Vector|GetForwardVector (Variables|Default|GetShipPivot))) false false))

(fn CatchWind
  (bind _windsource (Variables|Default|GetWindSource))
  (bind _shippivot (Variables|Default|GetShipPivot))
  (bind _returnvalue (Transformation|GetWorldLocation _shippivot))
  (bind _returnvalue_2 (Transformation|GetActorLocation _windsource))
  (bind _returnvalue_3 (Math|Vector|Normalize _returnvalue_2))
  (bind _returnvalue_4 (Math|Vector|Normalize _returnvalue))
  (bind _returnvalue_5 (* (.z _returnvalue_4) (.z _returnvalue_3)))
  (bind _returnvalue_6 (* (.x _returnvalue_4) (.x _returnvalue_3)))
  (bind _returnvalue_7 (* (.y _returnvalue_4) (.y _returnvalue_3)))
  (bind _returnvalue_8 (+ _returnvalue_6 _returnvalue_7 _returnvalue_5))
  (bind _returnvalue_9 (Class|KismetMathLibrary|DegAcos _returnvalue_8))
  ;[0.15 0.15 0.15 0.5] Setting Speed depending on angle on angle
  (Utilities|FlowControl|Sequence
    (:then_0
      (if (< _returnvalue_9 2e+01)
        (Variables|Default|SetMaxForwardSpeed 15.0)
        (Variables|Default|SetForwardAcceleration 1.5)
        (Development|PrintString "Top Speed")))
    (:then_1
      (if (and (> _returnvalue_9 21.0) (< _returnvalue_9 4e+01))
        (Variables|Default|SetMaxForwardSpeed 1e+01)
        (Variables|Default|SetForwardAcceleration 0.75)
        (Development|PrintString "mid speed")))
    (:then_2
      (if (> _returnvalue_9 41.0)
        (Variables|Default|SetMaxForwardSpeed 5.0)
        (Variables|Default|SetForwardAcceleration 0.5)
        (Development|PrintString "Lowest Speed")))))

(fn DetermineWindSide)